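; BP_TownChara is an actor, named as a town character, that follows a spline supplied by BpSplineActor.
; On BeginPlay it snaps to the spline transform at its Distance with zero speed.
; Each Tick it passes Distance and Speed scaled by delta time to GetSplineTransform, then applies the result without sweep.
; This graph never writes Distance itself.
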(event EventBeginPlay
  (bind _transform (Default|GetSplineTransform (Variables|Default|Getbp_SplineActor) (Variables|Default|Getdistance) 0.0))
  (Transformation|SetActorTransform _transform))

(event EventTick
  (params (DeltaSeconds :type Float%20%28single-precision%29))
  (bind _transform (Default|GetSplineTransform (Variables|Default|Getbp_SplineActor) (Variables|Default|Getdistance) (* DeltaSeconds (Variables|Default|Getspeed))))
  (Transformation|SetActorTransform _transform))

(fn ConstructionScript)