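; Player camera pawn with a visible mouse cursor, Enhanced Input movement and left-click destruction of the actor under the cursor.
; IA_Move follows control rotation, while IA_Zoom moves the pawn along the camera's forward vector.
; IA_Watch calls ShootLine to trace and print the hit actor's name, though the trace end scales camera location instead of forward vector.
; The Shoot event is an unused stub.
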(event Custom|Shoot
  (params (transform :type Transform)))

(event Input|EnhancedActionEvents|EnhancedInputActionIA_Zoom
  (params (ActionValue :type Vector%202D%20Structure) (ElapsedSeconds :type Float%20%28double-precision%29) (TriggeredSeconds :type Float%20%28double-precision%29) (InputAction :type Input%20Action%20Object%20Reference :default "/Game/Input/Actions/IA_Zoom.IA_Zoom"))
  (bind _camera (Variables|Default|GetCamera))
  (bind _returnvalue (Transformation|GetWorldRotation _camera))
  (Pawn|Input|AddMovementInput (Math|Vector|GetForwardVector _returnvalue) (.x ActionValue) false)
  (Pawn|Input|AddMovementInput (Math|Vector|GetForwardVector _returnvalue) (.y ActionValue) false))

(event Input|EnhancedActionEvents|EnhancedInputActionIA_Move
  (params (ActionValue :type Vector%202D%20Structure) (ElapsedSeconds :type Float%20%28double-precision%29) (TriggeredSeconds :type Float%20%28double-precision%29) (InputAction :type Input%20Action%20Object%20Reference :default "/Game/Input/Actions/IA_Move.IA_Move"))
  (bind _returnvalue (Pawn|GetControlRotation :!class /Script/Engine.Pawn))
  (Pawn|Input|AddMovementInput (Math|Vector|GetForwardVector _returnvalue) (.x ActionValue) false)
  (Pawn|Input|AddMovementInput (Math|Vector|GetRightVector _returnvalue) (.y ActionValue) false))

(event Input|EnhancedActionEvents|EnhancedInputActionIA_Watch
  (params (ActionValue :type Boolean) (ElapsedSeconds :type Float%20%28double-precision%29) (TriggeredSeconds :type Float%20%28double-precision%29) (InputAction :type Input%20Action%20Object%20Reference :default "/Game/Input/Actions/IA_Watch.IA_Watch"))
  (CallFunction|ShootLine))

(event EventBeginPlay
  (Utilities|FlowControl|Sequence
    (:then_0
      (Variables|/Script/Engine.PlayerController|SetbShowMouseCursor (Game|GetPlayerController 0) true)
      (Variables|/Script/Engine.PlayerController|SetbEnableClickEvents (Game|GetPlayerController 0) true)
      (Variables|/Script/Engine.PlayerController|SetbEnableMouseOverEvents (Game|GetPlayerController 0) true))
    (:then_1
      (Input|AddMappingContext (PlayerController|LocalPlayerSubsystems|GetEnhancedInputLocalPlayerSubsystem (Game|GetPlayerController 0)) "/Game/Input/IMC_Input.IMC_Input" 0 "(bIgnoreAllPressedKeysUntilRelease=True,bForceImmediately=False,bNotifyUserSettings=False)"))))

(event Input|MouseEvents|LeftMouseButton
  (params (Key :type Key%20Structure :default "None"))
  (:Pressed
    (bind _hitresult (Game|Player|GetHitResultUnderCursorbyChannel (Game|GetPlayerController 0) "TraceTypeQuery1" true))
    (bind _hitactor (Collision|BreakHitResult _hitresult))
    (if (Utilities|IsValid _hitactor)
      (Actor|DestroyActor _hitactor))))

(fn ConstructionScript)

(fn ShootLine
  (bind _outhit (Collision|LineTraceByChannel (Transformation|GetWorldLocation (Variables|Default|GetCamera)) (+ (Math|Vector|GetForwardVector (Variables|Default|GetCamera)) (* (Transformation|GetWorldLocation (Variables|Default|GetCamera)) "1000.000000,1000.000000,1000.000000")) "TraceTypeQuery1" false 0 "None"))
  (Development|PrintString (Utilities|GetDisplayName (.hitactor _outhit))))